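; BP_Propeller models a drone propeller, turning an input value into thrust, RPM and weight figures.
; An InputValueChanged event scales input by max thrust and efficiency, derives RPM as the square root of thrust over constant K, and computes weight from mass and gravity.
; On BeginPlay it initializes with zero input and adds a WBP_PropelerDebugger widget bound to itself to the viewport.
; It only computes values; no force is applied here.
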(event `self.ReceiveBeginPlay`
  (`self.InputValueChanged` 0.0)
  (bind _returnvalue (`|CreateWidget` "/Game/PhysicsDrone/Blueprints/Testing/WBP_PropelerDebugger.WBP_PropelerDebugger_C" null self))
  (bind _output_get (set `self.DebugWidget` _returnvalue))
  (`UserWidget.AddToViewport` _output_get 0))

(event `InputValueChanged`
  (params (Value :type "Float (double-precision)"))
  (bind _output_get (set `self.InputThrust` (`self.ConvertInputToThrust` Value)))
  (set `self.RPM` (`self.CalculateRPM` _output_get))
  (set `self.Weight` (`self.CalculateWeight` (`self.Mass`))))

(fn `CalculateRPM`
  (params (Thrust :type "Float (double-precision)"))
  (returns (RPM :type "Float (double-precision)"))
  (return (`KismetMathLibrary.Sqrt` (/ Thrust (`self.k`)))))

(fn `CalculateWeight`
  (params (Mass :type "Float (double-precision)"))
  (returns (Weight :type "Float (double-precision)"))
  (return (* Mass (`self.GravitationalConstant`))))

(fn `ConvertInputToThrust`
  (params (ThrustFromInput :type "Float (double-precision)"))
  (returns (Thrust :type "Float (double-precision)"))
  (return (* ThrustFromInput (`self.MaxThrust`) (`self.PropellerEfficiency`))))

(fn `UserConstructionScript`)