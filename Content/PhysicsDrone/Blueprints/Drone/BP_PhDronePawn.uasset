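; Player-controlled physics drone pawn that adds its Enhanced Input mapping and possesses itself on BeginPlay.
; The thrust/yaw action feeds raw Y into SetThrottleInput; yaw, pitch and roll setters are unconnected, so pitch/roll input is only printed.
; Input values and the DroneMovementComponent's controls, read every tick, print on screen for debugging.
; A debug key applies an upward acceleration to the drone mesh's Root bone.
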(event Input|EnhancedActionEvents|EnhancedInputActionIA_ThrustYaw
  (params (ActionValue :type Vector%202D%20Structure) (ElapsedSeconds :type Float%20%28double-precision%29) (TriggeredSeconds :type Float%20%28double-precision%29) (InputAction :type Input%20Action%20Object%20Reference :default "/Game/PhysicsDrone/Blueprints/Inputs/IA_ThrustYaw.IA_ThrustYaw"))
  (bind (_x _y) (Math|Vector2D|BreakVector2D ActionValue))
  (Development|PrintString (Utilities|String|ToString(Text) (Utilities|Text|FormatText "{InputAction}->X: {X}, Y: {Y} " (Utilities|GetDisplayName InputAction) _x (Math|Float|Clamp(Float) _y))) true false "(R=0.000000,G=0.660000,B=1.000000,A=1.000000)" 0.0 "3")
  (Class|PhDronePawn|SetThrottleInput _y))

(event Input|EnhancedActionEvents|EnhancedInputActionIA_PitchRoll
  (params (ActionValue :type Vector%202D%20Structure) (ElapsedSeconds :type Float%20%28double-precision%29) (TriggeredSeconds :type Float%20%28double-precision%29) (InputAction :type Input%20Action%20Object%20Reference :default "/Game/PhysicsDrone/Blueprints/Inputs/IA_PitchRoll.IA_PitchRoll"))
  (bind (_x _y) (Math|Vector2D|BreakVector2D ActionValue))
  (Development|PrintString (Utilities|String|ToString(Text) (Utilities|Text|FormatText "{InputAction}->X: {X}, Y: {Y} " (Utilities|GetDisplayName InputAction) _x _y)) true false "(R=0.000000,G=0.660000,B=1.000000,A=1.000000)" 0.0 "4"))

(event EventBeginPlay
  (bind _returnvalue (Game|GetPlayerController 0))
  (bind _self self)
  (Input|AddMappingContext (PlayerController|LocalPlayerSubsystems|GetEnhancedInputLocalPlayerSubsystem _returnvalue) "/Game/PhysicsDrone/Blueprints/Inputs/IMC_DroneDefault.IMC_DroneDefault" 0 "(bIgnoreAllPressedKeysUntilRelease=True,bForceImmediately=False,bNotifyUserSettings=False)")
  (Pawn|Possess _returnvalue _self)
  (Input|EnableInput _self _returnvalue))

(event EventTick
  (params (DeltaSeconds :type Float%20%28single-precision%29))
  (bind _returnvalue (Class|PhysicsFloatingMovementComponent|GetControls (Variables|Default|GetDroneMovementComponent)))
  (Development|PrintString (Utilities|String|ToString(Text) (Utilities|Text|FormatText "{X}, {Y}, {Z}, {W} " (.X (Math|Vector4|BreakVector4 _returnvalue)) (.Y (Math|Vector4|BreakVector4 _returnvalue)) (.Z (Math|Vector4|BreakVector4 _returnvalue)) (.W (Math|Vector4|BreakVector4 _returnvalue)))) true false "(R=0.000000,G=0.660000,B=1.000000,A=1.000000)" 0.0 "5"))

(event Input|KeyboardEvents|DebugKeyAdd
  (params (Key :type Key%20Structure :default "None") (ActionValue :type Input%20Action%20Value%20Structure))
  (:Pressed
    (Physics|AddForce (Variables|Default|GetDroneMeshComponent) "0.000000,0.000000,50000.000000" "Root" true)))

(fn ConstructionScript)